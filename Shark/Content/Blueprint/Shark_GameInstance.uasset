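; Game instance for a shark game that sets up the save game at startup and restores the coin count.
; On Init it either loads slot "Test" and copies Coin into SharkGameMode, or creates and saves a fresh Shark_GameSave.
; The save object is kept in SaveGameData.
; The existence check queries an empty slot name, while loading and saving use "Test".
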(event EventInit
  (bind _returnvalue (SaveGame|DoesSaveGameExist))
  (if _returnvalue
    (Development|PrintString "SaveGame Exist")
    (bind _returnvalue_2 (SaveGame|LoadGamefromSlot "Test"))
    (bind _asshark_game_save (Utilities|Casting|CastToShark_GameSave _returnvalue_2))
    (bind _output_get (Variables|Default|SetSaveGameData _asshark_game_save))
    (bind _asshark_game_mode (Utilities|Casting|CastToSharkGameMode (Game|GetGameMode)))
    (Variables|/Game/GameMode/SharkGameMode.SharkGameMode_C|SetCoin _asshark_game_mode (Variables|/Game/Blueprint/Shark_GameSave.Shark_GameSave_C|GetCoin _output_get))
    (else
      (Development|PrintString "SaveDoesn't Exist")
      (bind _returnvalue_3 (SaveGame|CreateSaveGameObject "/Game/Blueprint/Shark_GameSave.Shark_GameSave_C"))
      (bind _output_get_2 (Variables|Default|SetSaveGameData _returnvalue_3))
      (SaveGame|SaveGametoSlot _output_get_2 "Test")
      (Development|PrintString "Save Success"))))