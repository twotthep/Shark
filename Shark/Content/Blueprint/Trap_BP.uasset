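; Trap actor that penalizes a ThirdPersonCharacter on overlap and then destroys itself.
; It consumes the character's shield if IsShield is set, otherwise applies damage.
; Either way it halves the character's CurrentFreefall.
; A Sequence calls DestroyActor before a delayed branch meant to restore CurrentFreefall, so that restore is scheduled on an actor already being destroyed.
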(event EventBeginPlay
  (Utilities|Casting|CastToSharkGameMode (Game|GetGameMode)))

(event Collision|EventActorBeginOverlap
  (params (OtherActor :type Actor%20Object%20Reference))
  (bind _asthird_person_character (Utilities|Casting|CastToThirdPersonCharacter OtherActor))
  (if (Variables|/Game/Blueprint/ThirdPersonCharacter.ThirdPersonCharacter_C|GetisShield _asthird_person_character)
    (Variables|/Game/Blueprint/ThirdPersonCharacter.ThirdPersonCharacter_C|SetisShield _asthird_person_character false)
    (else
      (Game|Damage|ApplyDamage _asthird_person_character 1.0 0 0)))
  (Variables|/Game/Blueprint/ThirdPersonCharacter.ThirdPersonCharacter_C|SetcurrentFreefall _asthird_person_character (* (Variables|/Game/Blueprint/ThirdPersonCharacter.ThirdPersonCharacter_C|GetcurrentFreefall _asthird_person_character) 0.5))
  (Utilities|FlowControl|Sequence
    (:then_0
      (Actor|DestroyActor))
    (:then_1
      (Utilities|FlowControl|Delay 2.0)
      (Variables|/Game/Blueprint/ThirdPersonCharacter.ThirdPersonCharacter_C|SetcurrentFreefall _asthird_person_character (/ (Variables|/Game/Blueprint/ThirdPersonCharacter.ThirdPersonCharacter_C|GetcurrentFreefall _asthird_person_character) 0.5))
      (Development|PrintString "Done: Delay Force"))))

(event EventTick
  (params (DeltaSeconds :type Float%20%28single-precision%29)))

(fn ConstructionScript)